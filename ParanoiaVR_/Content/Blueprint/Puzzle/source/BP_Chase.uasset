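; BP_Chase is an AI pawn that wanders at random and moves toward pawns it sees.
; From BeginPlay, RandomWonder moves it to random reachable points within a radius of its current location, repeating after a short delay.
; PawnSensing starts an AIMoveTo toward the seen pawn, then resumes wandering on success.
; Neither move handles failure, so a failed move does not itself restart wandering.
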(event OnSeePawn(PawnSensing)
  (params (Pawn :type Pawn%20Object%20Reference))
  (AI|AIMoveTo self "0, 0, 0" Pawn 5.0 false
    (:then
      (Utilities|FlowControl|Delay 0.2)
      (CallFunction|RandomWonder))))

(event Custom|RandomWonder
  (AI|AIMoveTo self (.RandomLocation (AI|Navigation|GetRandomReachablePointinRadius (Transformation|GetActorLocation) 1e+03 0 0)) 0 5.0 false
    (:then
      (Utilities|FlowControl|Delay 0.2)
      (CallFunction|RandomWonder))))

(event EventBeginPlay
  (CallFunction|RandomWonder))

(fn ConstructionScript)